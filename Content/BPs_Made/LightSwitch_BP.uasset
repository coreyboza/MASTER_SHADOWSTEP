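; One-shot light switch that lets the player turn off a linked static spotlight.
; ThirdPersonCharacter overlap shows prompt text and enables input only while SwitchedOn is set, then clears it, so only the first entry arms the switch.
; Interact plays a sound, zeroes the light, disables its cone collision and sets CanCutScene.
; Tick rotates the whole actor along the camera-to-text direction; rotating-light toggle logic is unconnected.
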(event EventTick
  (params (DeltaSeconds :type Float%20%28single-precision%29))
  ;[0 1 0.0615] text facing camera
  (Transformation|SetActorRotation (Math|Rotator|MakeRotfromX (- (Transformation|GetWorldLocation (Variables|Default|GetTexts)) (Transformation|GetActorLocation (Game|GetPlayerCameraManager 0))))))

(event Collision|EventActorEndOverlap
  (params (OtherActor :type Actor%20Object%20Reference))
  (Utilities|Casting|CastToThirdPersonCharacter OtherActor)
  (Variables|Default|SetIn%20Trigger false)
  (if (Variables|Default|GetIn%20Trigger)
    (if (Variables|Default|GetSwitchedOn)
      (Rendering|SetVisibility (Variables|Default|GetTexts) true false)
      (Variables|Default|SetFlipSwitch true)
      (Input|EnableInput (Game|GetPlayerController 0))
      (Variables|Default|SetSwitchedOn false)
      (else
        (Rendering|SetVisibility (Variables|Default|GetTexts) false false)))
    (else
      (Rendering|SetVisibility (Variables|Default|GetTexts) false false)
      (Variables|Default|SetFlipSwitch false)
      (Input|DisableInput (Game|GetPlayerController 0) 0))))

(event Collision|EventActorBeginOverlap
  (params (OtherActor :type Actor%20Object%20Reference))
  (Utilities|Casting|CastToThirdPersonCharacter OtherActor)
  (Variables|Default|SetIn%20Trigger true)
  (if (Variables|Default|GetIn%20Trigger)
    (if (Variables|Default|GetSwitchedOn)
      (Rendering|SetVisibility (Variables|Default|GetTexts) true false)
      (Variables|Default|SetFlipSwitch true)
      (Input|EnableInput (Game|GetPlayerController 0))
      (Variables|Default|SetSwitchedOn false)
      (else
        (Rendering|SetVisibility (Variables|Default|GetTexts) false false)))
    (else
      (Rendering|SetVisibility (Variables|Default|GetTexts) false false)
      (Variables|Default|SetFlipSwitch false)
      (Input|DisableInput (Game|GetPlayerController 0) 0))))

(event Input|ActionEvents|InputActionInteract
  (params (Key :type Key%20Structure))
  ;[1 0.4717 0] this is the only input for the light, one time use
  (:Pressed
    (if (Variables|Default|GetFlipSwitch)
      (Utilities|FlowControl|DoOnce false
        (:Completed
          (Audio|PlaySoundatLocation "/Game/Assets/Sound/lightSwitch.lightSwitch" "0, 0, 0")
          (Rendering|Components|Light|SetIntensity (Variables|/Script/Engine.SpotLight|GetSpotLightComponent (Variables|Default|GetStaticLightToBeFlopped)) 0.0)
          (Collision|SetCollisionEnabled (Variables|/Game/BPs_Made/StaticLight.StaticLight_C|GetCone (Variables|Default|GetStaticLightToBeFlopped)) "NoCollision")
          (Variables|/Game/BPs_Made/StaticLight.StaticLight_C|SetswitchedOn (Variables|Default|GetStaticLightToBeFlopped) false)
          (Rendering|SetVisibility (Variables|Default|GetTexts) false false)
          (Variables|Default|SetCanCutScene true))))))

(fn ConstructionScript)